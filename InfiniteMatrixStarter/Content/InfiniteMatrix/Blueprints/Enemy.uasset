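; Enemy actor for the InfiniteMatrix game that removes itself after a short lifespan.
; Its Box overlap destroys both the enemy and any Projectile it meets, and increments the score on the player pawn.
; Overlapping a BP_Player instead makes that player take damage and destroys the enemy.
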(event OnComponentBeginOverlap(Box)
  (params (OverlappedComponent :type Primitive%20Component%20Object%20Reference) (OtherActor :type Actor%20Object%20Reference) (OtherComp :type Primitive%20Component%20Object%20Reference) (OtherBodyIndex :type Integer) (bFromSweep :type Boolean) (SweepResult :type Hit%20Result%20Structure%20%28by%20ref%29))
  (bind _asprojectile (Utilities|Casting|CastToProjectile OtherActor)
    (:then
      (Utilities|FlowControl|Sequence
        (:then_0
          (Actor|DestroyActor)
          (bind _asbp_player (Utilities|Casting|CastToBP_Player (Game|Player|GetPlayerPawn 0)))
          (Default|IncrementScore _asbp_player))
        (:then_1
          (Actor|DestroyActor _asprojectile))))
    (:CastFailed
      (bind _asbp_player_2 (Utilities|Casting|CastToBP_Player OtherActor))
      (Default|TakeDamage _asbp_player_2)
      (Actor|DestroyActor))))

(event EventBeginPlay
  (Actor|SetLifeSpan 8.0))

(event Collision|EventActorBeginOverlap
  (params (OtherActor :type Actor%20Object%20Reference)))

(event EventTick
  (params (DeltaSeconds :type Float%20%28single-precision%29)))

(fn ConstructionScript)